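; BP_ChallengeCharcter is a playable challenge character with camera-relative movement, lives and death handling.
; Enhanced Input drives movement and look, and the IA_Speace action sets an IsRoll flag.
; Tick calls Dead below a height threshold, as does LoseHP when lives run out, ragdolling the mesh and disabling movement.
; An auto-death countdown timer feeds LoseHP, but nothing in this graph starts it.
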(event `自动死亡`
  ; 自动死亡
  (bind _returnvalue (`KismetSystemLibrary.K2_SetTimerDelegate` (delegate `自定义事件`) 1.0 true))
  (set `self.Timer` _returnvalue))

(event `自定义事件`
  ; 自动死亡
  (bind _output_get (set `self.DeadTime` (- (`self.DeadTime`) 1)))
  (if (<= _output_get 0)
    (`self.LoseHP`)
    (`KismetSystemLibrary.PrintString` (`KismetStringLibrary.Conv_IntToString` (`self.LiveNum`)))))

(event `self.ReceiveBeginPlay`
  ; 控制输入
  (`EnhancedInputSubsystemInterface.AddMappingContext` (pcsubsystem `EnhancedInputLocalPlayerSubsystem` (`GameplayStatics.GetPlayerController` 0)) "/Game/Code/Character/Input/IMC_ChallengeCharcter.IMC_ChallengeCharcter" 0 (struct)))

(event `EnhancedInput|/Game/Code/Character/Input/IA_Move`
  (params (ActionValue :type "Vector2D Structure") (ElapsedSeconds :type "Float (double-precision)") (TriggeredSeconds :type "Float (double-precision)") (InputAction :type "InputAction Object Reference" :default "/Game/Code/Character/Input/IA_Move.IA_Move"))
  (bind (_x _y) (`KismetMathLibrary.BreakVector2D` ActionValue))
  (bind (_returnvalue_roll _returnvalue_pitch _returnvalue_yaw) (`KismetMathLibrary.BreakRotator` (`SceneComponent.K2_GetComponentRotation` (`self.Camera`))))
  (bind (_returnvalue_roll_2 _returnvalue_pitch_2 _returnvalue_yaw_2) (`KismetMathLibrary.BreakRotator` (`SceneComponent.K2_GetComponentRotation` (`self.Camera`))))
  ; 前后左右移动
  (:`Triggered`
    (`self.AddMovementInput` (`KismetMathLibrary.GetForwardVector` (`KismetMathLibrary.MakeRotator` 0.0 0.0 _returnvalue_yaw)) _x)
    (`self.AddMovementInput` (`KismetMathLibrary.GetRightVector` (`KismetMathLibrary.MakeRotator` 0.0 0.0 _returnvalue_yaw_2)) _y)))

(event `EnhancedInput|/Game/Code/Character/Input/IA_Look`
  (params (ActionValue :type "Vector2D Structure") (ElapsedSeconds :type "Float (double-precision)") (TriggeredSeconds :type "Float (double-precision)") (InputAction :type "InputAction Object Reference" :default "/Game/Code/Character/Input/IA_Look.IA_Look"))
  (bind (_x _y) (`KismetMathLibrary.BreakVector2D` ActionValue))
  ; 鼠标控制视野
  (:`Triggered`
    (`self.AddControllerYawInput` _x)
    (`self.AddControllerPitchInput` _y)))

(event `EnhancedInput|/Game/Code/Character/Input/IA_Speace`
  (params (ActionValue :type Boolean) (ElapsedSeconds :type "Float (double-precision)") (TriggeredSeconds :type "Float (double-precision)") (InputAction :type "InputAction Object Reference" :default "/Game/Code/Character/Input/IA_Speace.IA_Speace"))
  (:`Started`
    (set `self.IsRoll` ActionValue))
  (:`Completed`
    (set `self.IsRoll` ActionValue)))

(event `/Game/Code/Message/BPI_Dead.Dead`
  ; Dead
  (`PrimitiveComponent.SetSimulatePhysics` (`self.Mesh`) true)
  (set `SpringArmComponent.bDoCollisionTest` false (`self.SpringArm`))
  (`CharacterMovementComponent.SetMovementMode` (`self.CharacterMovement`) "MOVE_None" 0))

(event `LoseHP`
  ; 减少血量
  (bind _output_get (set `self.LiveNum` (- (`self.LiveNum`) 1)))
  (if (not (> _output_get 0))
    (`self.Dead`)))

(event `self.ReceiveTick`
  (params (DeltaSeconds :type "Float (single-precision)"))
  (bind (_returnvalue_x _returnvalue_y _returnvalue_z) (`KismetMathLibrary.BreakVector` (`self.K2_GetActorLocation`)))
  ; 检测是否掉入坑里
  (if (<= _returnvalue_z (`self.DeadHeight`))
    (`self.Dead`)))

(fn `UserConstructionScript`)