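; BP_ChallengeCharcter is the player character for a challenge mode, with Enhanced Input movement, look and jump.
; BeginPlay adds the challenge mapping context, and movement follows the camera's forward and right vectors.
; Tick calls Dead whenever the character drops to a fixed water-death height.
; Dead ragdolls the mesh, disables spring arm collision and movement, then after a delay destroys the actor and calls Rebirth on BP_ChallengeMode.
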(event `self.ReceiveBeginPlay`
  ; 绑定事件
  (`EnhancedInputSubsystemInterface.AddMappingContext` (pcsubsystem `EnhancedInputLocalPlayerSubsystem` (`GameplayStatics.GetPlayerController` 0)) "/Game/Code/Character/Input/IMC_Challenge.IMC_Challenge" 0 (struct)))

(event `EnhancedInput|/Game/Code/Character/Input/IA_Move`
  (params (ActionValue :type "Vector2D Structure") (ElapsedSeconds :type "Float (double-precision)") (TriggeredSeconds :type "Float (double-precision)") (InputAction :type "InputAction Object Reference" :default "/Game/Code/Character/Input/IA_Move.IA_Move"))
  (bind (_x _y) (`KismetMathLibrary.BreakVector2D` ActionValue))
  ; 控制移动
  (:`Triggered`
    (`self.AddMovementInput` (`SceneComponent.GetForwardVector` (`self.Camera`)) _x)
    (`self.AddMovementInput` (`SceneComponent.GetRightVector` (`self.Camera`)) _y)))

(event `EnhancedInput|/Game/Code/Character/Input/IA_Look`
  (params (ActionValue :type "Vector2D Structure") (ElapsedSeconds :type "Float (double-precision)") (TriggeredSeconds :type "Float (double-precision)") (InputAction :type "InputAction Object Reference" :default "/Game/Code/Character/Input/IA_Look.IA_Look"))
  (bind (_x _y) (`KismetMathLibrary.BreakVector2D` ActionValue))
  ; 控制视角
  (:`Triggered`
    (`self.AddControllerYawInput` _x)
    (`self.AddControllerPitchInput` _y)))

(event `EnhancedInput|/Game/Code/Character/Input/IA_Jump`
  (params (ActionValue :type Boolean) (ElapsedSeconds :type "Float (double-precision)") (TriggeredSeconds :type "Float (double-precision)") (InputAction :type "InputAction Object Reference" :default "/Game/Code/Character/Input/IA_Jump.IA_Jump"))
  ; 跳跃
  (:`Started`
    (`self.Jump`)))

(event `Dead`
  ; 死亡
  (`PrimitiveComponent.SetSimulatePhysics` (`self.Mesh`) true)
  (set `SpringArmComponent.bDoCollisionTest` false (`self.PlayerSpringArm`))
  (`CharacterMovementComponent.SetMovementMode` (`self.CharacterMovement`) "MOVE_None" 0)
  (`KismetSystemLibrary.Delay` 2.0)
  (`self.K2_DestroyActor`)
  (bind _asbp_challenge_mode (cast `/Game/Code/Character/BP_ChallengeMode` (`GameplayStatics.GetGameMode`)))
  (`/Game/Code/Character/BP_ChallengeMode.Rebirth` _asbp_challenge_mode))

(event `self.ReceiveTick`
  (params (DeltaSeconds :type "Float (single-precision)"))
  (bind (_returnvalue_x _returnvalue_y _returnvalue_z) (`KismetMathLibrary.BreakVector` (`self.K2_GetActorLocation`)))
  ; 检测落水死亡-检查Z轴是否小于452
  (if (<= _returnvalue_z 452.0)
    (`self.Dead`)))

(fn `UserConstructionScript`)