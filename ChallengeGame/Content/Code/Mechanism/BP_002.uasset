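; BP_002 is a mechanism actor that moves two wooden pole meshes vertically when play begins.
; On BeginPlay it caches both poles' relative locations, then a timeline track drives one pole's Z offset directly and the other by the absolute difference from 150, so they move in opposition.
; A Dead event only prints a debug "Hello" string.
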(event `self.ReceiveBeginPlay`
  (bind (_location08_x _location08_y _location08_z) (`KismetMathLibrary.BreakVector` (`self.Location08`)))
  (bind (_location06_x _location06_y _location06_z) (`KismetMathLibrary.BreakVector` (`self.Location06`)))
  (set `self.Location06` (`SceneComponent.RelativeLocation` (`self.SM_WoodenPole_06`)))
  (set `self.Location08` (`SceneComponent.RelativeLocation` (`self.SM_WoodenPole_08`)))
  (bind (_direction `_新建轨道_0`) (`Timeline|时间轴`)
    (:`Update`
      (`SceneComponent.K2_SetRelativeLocation` (`self.SM_WoodenPole_06`) (`KismetMathLibrary.MakeVector` _location06_x _location06_y (+ _location06_z `_新建轨道_0`)) false false)
      (`SceneComponent.K2_SetRelativeLocation` (`self.SM_WoodenPole_08`) (`KismetMathLibrary.MakeVector` _location08_x _location08_y (+ _location08_z (`KismetMathLibrary.Abs` (- `_新建轨道_0` 150.0)))) false false))))

(event `/Game/Code/BlueprintInterface/BPI_Dead.Dead`
  (`KismetSystemLibrary.PrintString` "Hello"))

(fn `UserConstructionScript`)