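; BP_003 is a rotating obstacle mechanism that either kills or knocks away the challenge character on contact.
; Tick spins the Body around yaw by a variable amount per frame, without delta-time scaling.
; When the Capsule overlaps a BP_ChallengeCharcter, the Death flag selects between calling Dead and applying a strong impulse along the Arrow's forward vector.
; The construction script shows the Thorn component only when Death is set.
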(event `self.ReceiveTick`
  (params (DeltaSeconds :type "Float (single-precision)"))
  ; 添加旋转功能
  (`SceneComponent.K2_AddRelativeRotation` (`self.Body`) (`KismetMathLibrary.MakeRotator` 0.0 0.0 (`self.Delta Rotation Z (Yaw)`)) false false))

(event `self.Capsule.OnComponentBeginOverlap`
  (params (OverlappedComponent :type "PrimitiveComponent Object Reference") (OtherActor :type "Actor Object Reference") (OtherComp :type "PrimitiveComponent Object Reference") (OtherBodyIndex :type Integer) (bFromSweep :type Boolean) (SweepResult :type "HitResult Structure (by ref)"))
  ; 添加死亡和击飞效果
  (bind _asbp_challenge_charcter (cast `/Game/Code/Character/BP_ChallengeCharcter` OtherActor))
  (if (`self.Death`)
    (`/Game/Code/Character/BP_ChallengeCharcter.Dead` _asbp_challenge_charcter)
    (else
      (`CharacterMovementComponent.AddImpulse` (`Character.CharacterMovement` _asbp_challenge_charcter) (* (`SceneComponent.GetForwardVector` (`self.Arrow`)) 20000) false))))

(fn `UserConstructionScript`
  ; 通过变量Death来判断组件形态
  (if (`self.Death`)
    (`SceneComponent.SetVisibility` (`self.Thorn`) true false)
    (else
      (`SceneComponent.SetVisibility` (`self.Thorn`) false false))))