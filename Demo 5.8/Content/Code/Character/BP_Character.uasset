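; BP_Character is a player character Blueprint that handles basic look and movement through Enhanced Input.
; BeginPlay adds the IMC_Input mapping context to player 0's input subsystem.
; IA_Look2 feeds controller yaw and pitch.
; IA_Move2 drives movement along forward (X) and right (Y) vectors built from the camera's world yaw only, keeping motion camera-relative and horizontal regardless of pitch.
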(event `EnhancedInput|/Game/Code/Input/IA_Look2`
  (params (ActionValue :type "Vector2D Structure") (ElapsedSeconds :type "Float (double-precision)") (TriggeredSeconds :type "Float (double-precision)") (InputAction :type "InputAction Object Reference" :default "/Game/Code/Input/IA_Look2.IA_Look2"))
  (bind (_x _y) (`KismetMathLibrary.BreakVector2D` ActionValue))
  ; 角色视角旋转
  (:`Triggered`
    (`self.AddControllerYawInput` _x)
    (`self.AddControllerPitchInput` _y)))

(event `self.ReceiveBeginPlay`
  ; 绑定角色控制器
  (`EnhancedInputSubsystemInterface.AddMappingContext` (pcsubsystem `EnhancedInputLocalPlayerSubsystem` (`GameplayStatics.GetPlayerController` 0)) "/Game/Code/Input/IMC_Input.IMC_Input" 0 (struct)))

(event `EnhancedInput|/Game/Code/Input/IA_Move2`
  (params (ActionValue :type "Vector2D Structure") (ElapsedSeconds :type "Float (double-precision)") (TriggeredSeconds :type "Float (double-precision)") (InputAction :type "InputAction Object Reference" :default "/Game/Code/Input/IA_Move2.IA_Move2"))
  (bind (_x _y) (`KismetMathLibrary.BreakVector2D` ActionValue))
  (bind (_returnvalue_roll _returnvalue_pitch _returnvalue_yaw) (`KismetMathLibrary.BreakRotator` (`SceneComponent.K2_GetComponentRotation` (`self.Camera`))))
  (bind (_returnvalue_roll_2 _returnvalue_pitch_2 _returnvalue_yaw_2) (`KismetMathLibrary.BreakRotator` (`SceneComponent.K2_GetComponentRotation` (`self.Camera`))))
  ; 角色移动
  (:`Triggered`
    (`self.AddMovementInput` (`KismetMathLibrary.GetForwardVector` (`KismetMathLibrary.MakeRotator` 0.0 0.0 _returnvalue_yaw_2)) _x)
    (`self.AddMovementInput` (`KismetMathLibrary.GetRightVector` (`KismetMathLibrary.MakeRotator` 0.0 0.0 _returnvalue_yaw)) _y)))

(fn `UserConstructionScript`)